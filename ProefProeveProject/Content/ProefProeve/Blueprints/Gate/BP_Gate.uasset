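; BP_Gate is an interactable gate that opens only when the player character has a key.
; Looking at it toggles an indicator, yawed from the player's forward vector.
; Interacting requires a valid indicator and destroys it before the key check, even when locked.
; With the key, the gate animation plays and both doors lose collision; otherwise the crosshair widget briefly shows a lock.
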(event EventOnInteractionLookat
  (params (IsLookingAt :type Boolean))
  (bind _interactionindicator (Variables|Default|GetInteractionIndicator))
  ;[1 1 1 0.5] Show the interaction indicator towards the player
  (Utilities|IsValid _interactionindicator
    (:Is%20Valid
      (Rendering|SetVisibility _interactionindicator IsLookingAt true)
      (Transformation|SetWorldRotation (Variables|Default|GetInteractionIndicator) (Math|Rotator|MakeRotator 0.0 0.0 (+ (.yaw (Math|Conversions|RotationFromXVector (Transformation|GetActorForwardVector (Game|Player|GetPlayerPawn 0)))) 9e+01)) false false))))

(event EventOnInteract
  (bind _interactionindicator (Variables|Default|GetInteractionIndicator))
  ;[1 1 1 0.5] Play the opening animation and remove the collision
  (Utilities|IsValid _interactionindicator
    (:Is%20Valid
      (Components|DestroyComponent _interactionindicator)
      (bind _foundwidgets (Widget|GetAllWidgetsOfClass "/Game/ProefProeve/Blueprints/Widgets/WBP_Crosshair.WBP_Crosshair_C" true))
      (if (Variables|/Game/ProefProeve/Blueprints/Player/BP_PlayerCharacter.BP_PlayerCharacter_C|GetHasKey (.AsBP%20Player%20Character (Utilities|Casting|CastToBP_PlayerCharacter (Game|Player|GetPlayerPawn 0))))
        (Default|SwitchtoDefaultCrosshair (Utilities|Array|Get(acopy) _foundwidgets))
        (Components|Animation|PlayAnimation (Variables|Default|GetAS_Gate_L_gate) "/Game/ProefProeve/Art/GateHouse/Gate/RootNode_TrackSetNode.RootNode_TrackSetNode" false)
        (Collision|SetCollisionEnabled (Variables|Default|GetLeftDoor) "NoCollision")
        (Collision|SetCollisionEnabled (Variables|Default|GetRightDoor) "NoCollision")
        (else
          (Default|SwitchtoLockCrosshair (Utilities|Array|Get(acopy) _foundwidgets))
          (Utilities|FlowControl|Delay (Variables|Default|GetLockCrosshairDuration))
          (Default|SwitchtoDefaultCrosshair (Utilities|Array|Get(acopy) _foundwidgets)))))))

(fn ConstructionScript)