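; BP_Key is a key pickup that the player collects by interacting with it.
; Looking at it toggles the InteractionIndicator and sets its yaw from the player pawn's forward vector plus 90 degrees, turning it toward the player.
; On interaction it adds a WBP_KeySlot widget to the viewport, sets HasKey on BP_PlayerCharacter and destroys itself.
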(event EventOnInteractionLookat
  (params (IsLookingAt :type Boolean))
  ;[1 1 1 0.5] Show the interaction indicator towards the player
  (Rendering|SetVisibility (Variables|Default|GetInteractionIndicator) IsLookingAt true)
  (Transformation|SetWorldRotation (Variables|Default|GetInteractionIndicator) (Math|Rotator|MakeRotator 0.0 0.0 (+ (.yaw (Math|Conversions|RotationFromXVector (Transformation|GetActorForwardVector (Game|Player|GetPlayerPawn 0)))) 9e+01)) false false))

(event EventOnInteract
  ;[1 1 1 0.5] Add the key slot to the UI
  (bind _returnvalue (UserInterface|CreateWidget "/Game/ProefProeve/Blueprints/Widgets/WBP_KeySlot.WBP_KeySlot_C"))
  (UserInterface|Viewport|AddtoViewport _returnvalue 0)
  (Variables|/Game/ProefProeve/Blueprints/Player/BP_PlayerCharacter.BP_PlayerCharacter_C|SetHasKey (.AsBP%20Player%20Character (Utilities|Casting|CastToBP_PlayerCharacter (Game|Player|GetPlayerPawn 0))) true)
  (Actor|DestroyActor))

(fn ConstructionScript)