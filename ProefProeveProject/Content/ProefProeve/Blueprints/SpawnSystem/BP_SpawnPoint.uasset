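; BP_SpawnPoint is a placeable spawner that creates an actor of a configurable class at its root transform.
; It spawns on BeginPlay when SpawnOnStart is set, or whenever SpawnNewActor is called.
; With ShouldRespawn enabled, it binds to the spawned actor's OnDestroyed event and uses a timer to spawn a replacement after RespawnTime, repeating the cycle.
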(event Custom|SpawnNewActor
  (bind _returnvalue (Game|SpawnActorfromClass (Variables|Spawnable|GetClassToSpawn) (Transformation|GetWorldTransform (Variables|Default|GetDefaultSceneRoot)) "Undefined" "MultiplyWithRoot" 0 0))
  (if (Variables|Respawning|GetShouldRespawn)
    (Game|AssignOnDestroyed _returnvalue (delegate Custom|OnActorDestroyed_Event))))

(event Custom|OnActorDestroyed_Event
  (params (DestroyedActor :type Actor%20Object%20Reference))
  (Utilities|Time|SetTimerbyEvent (delegate Custom|RespawnActor) (Variables|Respawning|GetRespawnTime)))

(event Custom|RespawnActor
  (CallFunction|SpawnNewActor))

(event EventBeginPlay
  (if (Variables|Spawnable|GetSpawnOnStart)
    (CallFunction|SpawnNewActor)))

(fn ConstructionScript)