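; BP_EnemyController is the AI controller for enemies, running BT_Enemy and signalling roam or chase state through event dispatchers.
; It starts the tree and signals roam on BeginPlay.
; Any perception update for a BP_PlayerCharacter, without checking sensing success, writes the player to the TargetActor blackboard key and signals chase.
; A perception-forgotten event clears that key and signals roam again.
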(event OnTargetPerceptionUpdated(AIPerception)
  (params (Actor :type Actor%20Object%20Reference) (Stimulus :type AI%20Stimulus%20Structure))
  ;[1 1 1 0.5] When the perception is updated. Update the TargetActor blackboard value and call the Chase dispatcher
  (bind _asbp_player_character (Utilities|Casting|CastToBP_PlayerCharacter Actor))
  (AI|Components|Blackboard|SetValueasObject (AI|GetBlackboard 0) (Utilities|Name|MakeLiteralName "TargetActor") _asbp_player_character)
  (Default|CallOnChaseEvent))

(event OnTargetPerceptionForgotten(AIPerception)
  (params (Actor :type Actor%20Object%20Reference))
  ;[1 1 1 0.5] When the perception is forgotten. Clear the TargetActor blackboard value and call the Roam dispatcher
  (AI|Components|Blackboard|ClearValue (AI|GetBlackboard 0) (Utilities|Name|MakeLiteralName "TargetActor"))
  (Default|CallOnRoamEvent))

(event EventBeginPlay
  ;[1 1 1 0.5] Start the enemy's behavior tree and call the Roam dispatcher
  (AI|RunBehaviorTree "/Game/ProefProeve/Blueprints/Enemy/AI/BT_Enemy.BT_Enemy")
  (Default|CallOnRoamEvent))

(fn ConstructionScript)