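; Enemy actor Blueprint that plays sound cues in response to its AI controller's attack and chase events.
; On BeginPlay it finds the first BP_EnemyController in the level and binds to both events.
; Attack plays a jumpscare sound at the enemy's location.
; Chase spawns an attached zombie sound that repeats ten seconds after each playback finishes, with no check that the chase is still active.
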(event Custom|OnAttackEvent_Event
  (Audio|PlaySoundatLocation "/Game/ProefProeve/Art/SFX/SW_Jumpscare.SW_Jumpscare" (Transformation|GetActorLocation) "0, 0, 0" 1.0 1.0 0.0 0 0 0 0))

(event Custom|OnChaseEvent_Event
  (bind _returnvalue (Audio|SpawnSoundAttached "/Game/ProefProeve/Art/SFX/SW_Zombie_02.SW_Zombie_02" 0 "None" "0, 0, 0" "0, 0, 0" "KeepRelativeOffset" false 1.0 1.0 0.0 0 0))
  (EventDispatchers|AssignOnAudioFinished _returnvalue (delegate Custom|OnAudioFinished_Event)))

(event Custom|OnAudioFinished_Event
  (Utilities|Time|SetTimerbyEvent (delegate Custom|OnChaseEvent_Event) 1e+01))

(event EventBeginPlay
  (bind _returnvalue (Actor|GetActorOfClass "/Game/ProefProeve/Blueprints/Enemy/AI/BP_EnemyController.BP_EnemyController_C"))
  (bind _output_get (Variables|Default|SetAIController _returnvalue))
  (EventDispatchers|AssignOnAttackEvent _output_get (delegate Custom|OnAttackEvent_Event))
  (EventDispatchers|AssignOnChaseEvent (Variables|Default|GetAIController) (delegate Custom|OnChaseEvent_Event)))

(fn ConstructionScript)